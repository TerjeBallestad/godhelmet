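; Pilotable mining ship that the player possesses via Interact and leaves with Cancel, attaching and hiding the pawn meanwhile.
; Physics-driven flight sets linear velocity each tick from smoothed thrust with Sprint superspeed, and applies torque for pitch, roll and yaw.
; While piloted, overlap volumes enable mining the nearest asteroid on input and looting on touch.
; The low-speed upward velocity term evaluates to zero, and angular damping logic is unwired.
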(event OnComponentBeginOverlap(LootTrigger)
  (params (OverlappedComponent :type Primitive%20Component%20Object%20Reference) (OtherActor :type Actor%20Object%20Reference) (OtherComp :type Primitive%20Component%20Object%20Reference) (OtherBodyIndex :type Integer) (bFromSweep :type Boolean) (SweepResult :type Hit%20Result%20Structure%20%28by%20ref%29))
  (Class|Lootable|Loot(Message) OtherActor))

(event EventBeginPlay)

(event EventTick
  (params (DeltaSeconds :type Float%20%28single-precision%29))
  (Utilities|FlowControl|Sequence
    (:then_0
      (if (< (Math|Vector|VectorLength (Variables|Default|GetForwardVelocity)) (Variables|Default|GetGravityThreshold))
        (Variables|Default|SetUpwardVelocity (* (Math|Vector|UnrotateVector (Math|Vector|GetUpVector (Variables|Default|GetModel)) (Transformation|GetWorldRotation (Variables|Default|GetModel))) (Math|Float|Lerp 0.0 0.0 (- (Math|Vector|VectorLength (Variables|Default|GetForwardVelocity)) (Variables|Default|GetGravityThreshold)))))
        (else
          (Variables|Default|SetUpwardVelocity (Math|Interpolation|VInterpTo (Variables|Default|GetUpwardVelocity) "0, 0, 0" (Utilities|Time|GetWorldDeltaSeconds) 2e+01)))))
    (:then_1
      (Physics|SetPhysicsLinearVelocity (Variables|Default|GetModel) (+ (Variables|Default|GetForwardVelocity) (Variables|Default|GetUpwardVelocity)) false "None"))))

(event EventInteract
  (bind _returnvalue (Game|GetPlayerController 0))
  (bind _self self)
  (bind _returnvalue_2 (Pawn|GetControlledPawn _returnvalue))
  ;[1 1 1] Interaction
  (Transformation|AttachActorToActor _returnvalue_2 _self "None" "KeepWorld" "KeepWorld" "KeepWorld" true)
  (bind _output_get (Variables|Default|SetDriverPawn _returnvalue_2))
  (Pawn|Possess _returnvalue _self)
  (Development|PrintText (Utilities|Text|FormatText "Interacting with {name}" (Utilities|GetDisplayName self)))
  (Rendering|SetActorHiddenInGame _output_get true)
  (Collision|SetActorEnableCollision _output_get false)
  (Variables|/Script/Engine.PrimitiveComponent|SetbGenerateOverlapEvents (Variables|Default|GetMining) true)
  (Variables|/Script/Engine.PrimitiveComponent|SetbGenerateOverlapEvents (Variables|Default|GetLootTrigger) true)
  (Physics|SetEnableGravity (Variables|Default|GetModel) false))

(event Input|ActionEvents|InputActionSprint
  (params (Key :type Key%20Structure :default "None"))
  ;[1 1 1] Superspeed
  (:Pressed
    (Variables|Default|SetSuperspeed true))
  (:Released
    (Variables|Default|SetSuperspeed false)))

(event Input|ActionEvents|InputActionInteract
  (params (Key :type Key%20Structure :default "None"))
  (:Pressed
    (Class|Minable|Mine(Message) (.ReturnValue (Actor|FindNearestActor (Transformation|GetWorldLocation (Variables|Default|GetModel)) (Collision|GetOverlappingActors (Variables|Default|GetMining) "/Game/godhelmet/Prototype/Asteroid/BP_Asteroid.BP_Asteroid_C" :!class /Script/Engine.PrimitiveComponent))))))

(event Input|ActionEvents|InputActionCancel
  (params (Key :type Key%20Structure :default "None"))
  (bind _driverpawn (Variables|Default|GetDriverPawn))
  ;[1 1 1] Cancel
  (:Pressed
    (Transformation|DetachFromActor _driverpawn "KeepWorld" "KeepRelative" "KeepWorld")
    (Variables|Default|SetForwardVelocity "0, 0, 0")
    (Physics|SetPhysicsLinearVelocity (Variables|Default|GetModel) "0, 0, 0" false "None")
    (Pawn|Possess (Game|GetPlayerController 0) _driverpawn)
    (Rendering|SetActorHiddenInGame _driverpawn false)
    (Collision|SetActorEnableCollision _driverpawn true)
    (Variables|/Script/Engine.PrimitiveComponent|SetbGenerateOverlapEvents (Variables|Default|GetMining) false)
    (Variables|/Script/Engine.PrimitiveComponent|SetbGenerateOverlapEvents (Variables|Default|GetLootTrigger) false)))

(event Input|AxisEvents|InputAxisMoveForward
  (params (AxisValue :type Float%20%28single-precision%29))
  (Utilities|FlowControl|Sequence
    (:then_0
      (if (Variables|Default|GetSuperspeed)
        (Variables|Default|SetThrustFactor (Variables|Default|GetSuperspeedFactor))
        (else
          (Variables|Default|SetThrustFactor 1.0)))
      (if (not (Math|Float|NearlyEqual(Float) AxisValue 0.0 0.1))
        (Variables|Default|SetThrust (Math|Interpolation|FInterpTo (Variables|Default|GetThrust) (Math|Float|Lerp 0.0 (Variables|Default|GetMaxThrust) (* AxisValue (Variables|Default|GetThrustFactor))) (Utilities|Time|GetWorldDeltaSeconds) (Variables|Default|GetAcceleration)))))
    (:then_1
      (Variables|Default|SetForwardVelocity (* (Math|Vector|GetForwardVector (Variables|Default|GetModel)) (Variables|Default|GetThrust))))))

(event Input|AxisEvents|InputAxisMoveRight
  (params (AxisValue :type Float%20%28single-precision%29))
  (bind _model (Variables|Default|GetModel))
  (Variables|Default|SetAngularDampTimer 3.0)
  (Class|PrimitiveComponent|AddTorqueinDegrees _model (* (Math|Vector|GetUpVector _model) (* AxisValue (Variables|Default|GetYawTorque))) "None" true))

(event Input|AxisEvents|InputAxisTurn
  (params (AxisValue :type Float%20%28single-precision%29))
  (bind _model (Variables|Default|GetModel))
  (Variables|Default|SetAngularDampTimer 3.0)
  (bind _result (Math|Float|NegateFloat AxisValue)
    (:%20%20
      (Class|PrimitiveComponent|AddTorqueinDegrees _model (* (Math|Vector|GetForwardVector _model) (* _result (Variables|Default|GetRollTorque))) "None" true))))

(event Input|AxisEvents|InputAxisLookUp
  (params (AxisValue :type Float%20%28single-precision%29))
  (bind _model (Variables|Default|GetModel))
  (Variables|Default|SetAngularDampTimer 3.0)
  (Class|PrimitiveComponent|AddTorqueinDegrees _model (* (Math|Vector|GetRightVector _model) (* AxisValue (Variables|Default|GetPitchTorque))) "None" true))

(fn ConstructionScript)