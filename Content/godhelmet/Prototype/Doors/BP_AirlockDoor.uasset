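; BP_AirlockDoor is an automatic door that animates when a pawn enters its trigger volume and reverses when a pawn leaves.
; The AnimateDoor timeline drives the door mesh's Z scale directly through its SizeZ track, keeping X and Y unchanged, so the door resizes instead of moving.
; The starting Z scale is saved on BeginPlay but is not used in the animation.
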(event OnComponentBeginOverlap(Trigger)
  (params (OverlappedComponent :type Primitive%20Component%20Object%20Reference) (OtherActor :type Actor%20Object%20Reference) (OtherComp :type Primitive%20Component%20Object%20Reference) (OtherBodyIndex :type Integer) (bFromSweep :type Boolean) (SweepResult :type Hit%20Result%20Structure%20%28by%20ref%29))
  (bind _door (Variables|Default|GetDoor))
  (bind _relativescale3d (Variables|/Script/Engine.SceneComponent|GetRelativeScale3D _door))
  (Utilities|Casting|CastToPawn OtherActor)
  (bind _sizez (Timeline|AnimateDoor Play)
    (:Update
      (Transformation|SetRelativeScale3D _door (Math|Vector|MakeVector (.x _relativescale3d) (.y _relativescale3d) _sizez)))))

(event OnComponentEndOverlap(Trigger)
  (params (OverlappedComponent :type Primitive%20Component%20Object%20Reference) (OtherActor :type Actor%20Object%20Reference) (OtherComp :type Primitive%20Component%20Object%20Reference) (OtherBodyIndex :type Integer))
  (bind _door (Variables|Default|GetDoor))
  (bind _relativescale3d (Variables|/Script/Engine.SceneComponent|GetRelativeScale3D _door))
  (Utilities|Casting|CastToPawn OtherActor)
  (bind _sizez (Timeline|AnimateDoor Reverse)
    (:Update
      (Transformation|SetRelativeScale3D _door (Math|Vector|MakeVector (.x _relativescale3d) (.y _relativescale3d) _sizez)))))

(event EventBeginPlay
  (Variables|Default|SetInitialSizeZ (.z (Variables|/Script/Engine.SceneComponent|GetRelativeScale3D (Variables|Default|GetDoor)))))

(fn ConstructionScript)