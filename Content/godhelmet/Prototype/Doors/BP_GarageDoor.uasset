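; Garage door prototype that toggles between open and closed each time its Interact event fires.
; BeginPlay caches the door mesh's Y scale, and Interact plays or reverses the AnimateDoor timeline.
; The timeline's SizeY track multiplies that cached scale, so the door animates by scaling along local Y rather than moving or rotating.
; Each update also prints the current Y size as debug text.
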(event EventInteract
  (bind _doormesh (Variables|Default|GetDoorMesh))
  (bind _relativescale3d (Variables|/Script/Engine.SceneComponent|GetRelativeScale3D _doormesh))
  (bind _output_get (Variables|Default|SetOpen (not (Variables|Default|GetOpen))))
  (if _output_get
    (bind _sizey (Timeline|AnimateDoor Play)
      (:Update
        (Transformation|SetRelativeScale3D _doormesh (Math|Vector|MakeVector (.x _relativescale3d) (* _sizey (Variables|Default|GetDoorSizeY)) (.z _relativescale3d)))
        (Development|PrintText (Utilities|Text|FormatText "SizeY: {size}" (* _sizey (Variables|Default|GetDoorSizeY))) true true "(R=0.000000,G=0.660000,B=1.000000,A=1.000000)" 0.0)))
    (else
      (Timeline|AnimateDoor Reverse))))

(event EventBeginPlay
  (Variables|Default|SetDoorSizeY (.y (Variables|/Script/Engine.SceneComponent|GetRelativeScale3D (Variables|Default|GetDoorMesh)))))

(fn ConstructionScript)