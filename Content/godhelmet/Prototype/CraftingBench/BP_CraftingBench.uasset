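; BP_CraftingBench is a prototype crafting bench pawn that a player takes control of by interacting with it.
; Interact stores the interacting pawn and has its controller possess the bench, and pressing Interact again hands possession back to that pawn.
; Possession shows a cached crafting menu bound to the inventory component with cursor input, and unpossession restores game-only input.
; Jump is a debug action that adds a test item to the inventory.
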(event EventInteract
  (params (InteractingActor :type Actor%20Object%20Reference))
  (bind _aspawn (Utilities|Casting|CastToPawn InteractingActor))
  (bind _output_get (Variables|Default|SetInteractingPawn _aspawn))
  (Pawn|Possess (Pawn|GetController _output_get) self))

(event EventPossessed
  (params (NewController :type Controller%20Object%20Reference))
  (bind _asplayer_controller (Utilities|Casting|CastToPlayerController NewController))
  (if (Utilities|IsValid (Variables|Default|GetCraftingMenu))
    (UserInterface|Viewport|AddtoViewport (Variables|Default|GetCraftingMenu) 0)
    (else
      (bind _returnvalue (UserInterface|CreateWidget "/Game/godhelmet/Prototype/CraftingBench/WBP_CraftingMenu.WBP_CraftingMenu_C" _asplayer_controller (Variables|Default|GetBP_InventoryComponent) 5e+01))
      (bind _output_get (Variables|Default|SetCraftingMenu _returnvalue))
      (UserInterface|Viewport|AddtoViewport _output_get 0)))
  (Input|SetInputModeGameandUI _asplayer_controller 0 "DoNotLock" false)
  (Variables|/Script/Engine.PlayerController|SetbShowMouseCursor _asplayer_controller true))

(event EventUnpossessed
  (params (OldController :type Controller%20Object%20Reference))
  (bind _craftingmenu (Variables|Default|GetCraftingMenu))
  (if (Utilities|IsValid _craftingmenu)
    (Widget|RemovefromParent _craftingmenu))
  (bind _asplayer_controller (Utilities|Casting|CastToPlayerController OldController))
  (Input|SetInputModeGameOnly _asplayer_controller)
  (Variables|/Script/Engine.PlayerController|SetbShowMouseCursor _asplayer_controller false))

(event Input|ActionEvents|InputActionInteract
  (params (Key :type Key%20Structure :default "None"))
  (:Pressed
    (Pawn|Possess (Game|GetPlayerController 0) (Variables|Default|GetInteractingPawn))
    (Development|PrintString "Hello" :!label _label))
  (:Released
    (goto _label)))

(event Input|ActionEvents|InputActionJump
  (params (Key :type Key%20Structure :default "None"))
  (:Pressed
    (bind _returnvalue (Game|ConstructObjectfromClass (Variables|Default|GetTestCraftClass) self (Utilities|Struct|MakeIntPoint 3 3) "/Game/godhelmet/Images/M_Icon_TurningMachine.M_Icon_TurningMachine" 0 0))
    (bind _success (Default|TryAddItem (Variables|Default|GetBP_InventoryComponent) _returnvalue))
    (Development|PrintText (Utilities|Text|FormatText "Tty to add item {item} results in {success}" (Utilities|GetObjectName _returnvalue) _success))))

(fn ConstructionScript)